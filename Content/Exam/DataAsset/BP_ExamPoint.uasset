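; BP_ExamPoint is a collectible point pickup whose sphere material and point value come from its Data variable.
; On player overlap it adds the value and increments the character's collectible counters, then hides itself and disables collision.
; If every point collectible is gathered without reaching the winning score, it freezes the player, plays a death animation, then after a delay deletes the character and opens Lvl_ThirdPerson.
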(event `self.ReceiveBeginPlay`
  (`PrimitiveComponent.SetMaterial` (`self.MeshSphere`) 0 (`/Game/Exam/DataAsset/BPDA_ExamCollectibles.Material` (`self.Data`))))

(event `self.ReceiveActorBeginOverlap`
  (params (OtherActor :type "Actor Object Reference"))
  (bind _meshsphere (`self.MeshSphere`))
  (if (== (`GameplayStatics.GetObjectClass` OtherActor) "/Game/ThirdPerson/Blueprints/BP_ThirdPersonCharacter.BP_ThirdPersonCharacter_C")
    (bind _asbp_third_person_character (cast `/Game/ThirdPerson/Blueprints/BP_ThirdPersonCharacter` (`GameplayStatics.GetPlayerCharacter` 0)))
    (set `/Game/ThirdPerson/Blueprints/BP_ThirdPersonCharacter.ExamPoints` (+ (`/Game/ThirdPerson/Blueprints/BP_ThirdPersonCharacter.ExamPoints` _asbp_third_person_character) (`/Game/Exam/DataAsset/BPDA_ExamCollectibles.Value` (`self.Data`))) _asbp_third_person_character)
    (set `/Game/ThirdPerson/Blueprints/BP_ThirdPersonCharacter.ExamCollectiblesGathered` (+ (`/Game/ThirdPerson/Blueprints/BP_ThirdPersonCharacter.ExamCollectiblesGathered` _asbp_third_person_character) 1) _asbp_third_person_character)
    (set `/Game/ThirdPerson/Blueprints/BP_ThirdPersonCharacter.ExamPointsCollectiblesGathered` (+ (`/Game/ThirdPerson/Blueprints/BP_ThirdPersonCharacter.ExamPointsCollectiblesGathered` _asbp_third_person_character) 1) _asbp_third_person_character)
    (`SceneComponent.SetVisibility` _meshsphere false true)
    (`PrimitiveComponent.SetCollisionEnabled` _meshsphere "NoCollision")
    (`PrimitiveComponent.SetCollisionEnabled` (`self.CollisionSphere`) "NoCollision")
    (bind _asbp_third_person_character_2 (cast `/Game/ThirdPerson/Blueprints/BP_ThirdPersonCharacter` (`GameplayStatics.GetPlayerCharacter` 0)))
    (if (and (== (`/Game/ThirdPerson/Blueprints/BP_ThirdPersonCharacter.ExamPointsCollectiblesGathered` _asbp_third_person_character_2) (`/Game/ThirdPerson/Blueprints/BP_ThirdPersonCharacter.ExamTotalPointsCollectibles` _asbp_third_person_character_2)) (not (>= (`/Game/ThirdPerson/Blueprints/BP_ThirdPersonCharacter.ExamPoints` _asbp_third_person_character_2) (`/Game/ThirdPerson/Blueprints/BP_ThirdPersonCharacter.ExamWinPoints` _asbp_third_person_character_2))))
      (`CharacterMovementComponent.DisableMovement` (`Character.CharacterMovement` _asbp_third_person_character_2))
      (`SkeletalMeshComponent.PlayAnimation` (`Character.Mesh` _asbp_third_person_character_2) "/Game/Exam/Animations/ExamDeath.ExamDeath" false)
      (`KismetSystemLibrary.Delay` 3.0)
      (`/Game/ThirdPerson/Blueprints/BP_ThirdPersonCharacter.Delete` _asbp_third_person_character_2)
      (`GameplayStatics.OpenLevel` "Lvl_ThirdPerson"))))

(fn `UserConstructionScript`)