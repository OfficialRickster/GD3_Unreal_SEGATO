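; BP_ExamDoor is a door actor whose Cube appears or disappears based on exam flags in BP_ThirdPersonGameMode.
; Each Tick it casts the game mode and does nothing unless ExamDoorUnlock is true.
; While unlocked, ExamTriggerBoxActivated makes the Cube visible and solid; otherwise the Cube is hidden with collision disabled, opening the way.
; The state is polled every frame rather than event-driven.
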(event `self.ReceiveTick`
  (params (DeltaSeconds :type "Float (single-precision)"))
  (bind _cube (`self.Cube`))
  (bind _asbp_third_person_game_mode (cast `/Game/ThirdPerson/Blueprints/BP_ThirdPersonGameMode` (`GameplayStatics.GetGameMode`)))
  (if (`/Game/ThirdPerson/Blueprints/BP_ThirdPersonGameMode.ExamDoorUnlock` _asbp_third_person_game_mode)
    (if (`/Game/ThirdPerson/Blueprints/BP_ThirdPersonGameMode.ExamTriggerBoxActivated` _asbp_third_person_game_mode)
      (`SceneComponent.SetVisibility` _cube true true)
      (`PrimitiveComponent.SetCollisionEnabled` _cube "QueryAndPhysics")
      (else
        (`SceneComponent.SetVisibility` _cube false true)
        (`PrimitiveComponent.SetCollisionEnabled` _cube "NoCollision")))))

(fn `UserConstructionScript`)