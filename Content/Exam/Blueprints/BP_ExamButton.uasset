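; BP_ExamButton is a timed overlap button that, together with others, unlocks the exam door.
; Overlapping a red button turns it green and increments a counter shared through BP_ThirdPersonGameMode.
; When the counter reaches two, it sets the door-unlock flag and streams in ExamLevel without blocking.
; Otherwise it reverts to red and decrements the counter after TimeToActivate, unless the door has been unlocked meanwhile.
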(event `self.ReceiveBeginPlay`
  (`PrimitiveComponent.SetMaterial` (`self.Cube`) 0 "/Game/Exam/Materials/Mat_ExamRed.Mat_ExamRed")
  (bind _asbp_third_person_game_mode (cast `/Game/ThirdPerson/Blueprints/BP_ThirdPersonGameMode` (`GameplayStatics.GetGameMode`)))
  (set `/Game/ThirdPerson/Blueprints/BP_ThirdPersonGameMode.ExamCounter` 0 _asbp_third_person_game_mode))

(event `self.ReceiveActorBeginOverlap`
  (params (OtherActor :type "Actor Object Reference"))
  (if (== (`PrimitiveComponent.GetMaterial` (`self.Cube`) 0) "/Game/Exam/Materials/Mat_ExamRed.Mat_ExamRed")
    (bind _asbp_third_person_game_mode (cast `/Game/ThirdPerson/Blueprints/BP_ThirdPersonGameMode` (`GameplayStatics.GetGameMode`)))
    (if (not (`/Game/ThirdPerson/Blueprints/BP_ThirdPersonGameMode.ExamDoorUnlock` _asbp_third_person_game_mode))
      (`PrimitiveComponent.SetMaterial` (`self.Cube`) 0 "/Game/Exam/Materials/Mat_ExamGreen.Mat_ExamGreen")
      (bind _asbp_third_person_game_mode_2 (cast `/Game/ThirdPerson/Blueprints/BP_ThirdPersonGameMode` (`GameplayStatics.GetGameMode`)))
      (bind _output_get (set `/Game/ThirdPerson/Blueprints/BP_ThirdPersonGameMode.ExamCounter` (+ (`/Game/ThirdPerson/Blueprints/BP_ThirdPersonGameMode.ExamCounter` _asbp_third_person_game_mode_2) 1) _asbp_third_person_game_mode_2))
      (if (== _output_get 2)
        (set `/Game/ThirdPerson/Blueprints/BP_ThirdPersonGameMode.ExamDoorUnlock` true _asbp_third_person_game_mode_2)
        (`GameplayStatics.LoadStreamLevelBySoftObjectPtr` "/Game/Exam/Level/ExamLevel.ExamLevel" true)
        (else
          (`KismetSystemLibrary.Delay` (`self.TimeToActivate`))
          (bind _asbp_third_person_game_mode_3 (cast `/Game/ThirdPerson/Blueprints/BP_ThirdPersonGameMode` (`GameplayStatics.GetGameMode`)))
          (if (not (`/Game/ThirdPerson/Blueprints/BP_ThirdPersonGameMode.ExamDoorUnlock` _asbp_third_person_game_mode_3))
            (set `/Game/ThirdPerson/Blueprints/BP_ThirdPersonGameMode.ExamCounter` (+ (`/Game/ThirdPerson/Blueprints/BP_ThirdPersonGameMode.ExamCounter` _asbp_third_person_game_mode_3) -1) _asbp_third_person_game_mode_3)
            (`PrimitiveComponent.SetMaterial` (`self.Cube`) 0 "/Game/Exam/Materials/Mat_ExamRed.Mat_ExamRed")))))))

(fn `UserConstructionScript`)