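; BP_ExamTriggerBox is a trigger that flags the exam as activated and records the level's collectible totals.
; On any actor overlap, it sets ExamTriggerBoxActivated on the third-person game mode.
; It then counts all BP_ExamPoint and BP_ExamPoison actors and writes point, poison and combined totals to player 0's character.
; The overlapping actor is not checked, and the counts are retaken on every overlap.
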(event `self.ReceiveActorBeginOverlap`
  (params (OtherActor :type "Actor Object Reference"))
  (bind _asbp_third_person_game_mode (cast `/Game/ThirdPerson/Blueprints/BP_ThirdPersonGameMode` (`GameplayStatics.GetGameMode`)))
  (set `/Game/ThirdPerson/Blueprints/BP_ThirdPersonGameMode.ExamTriggerBoxActivated` true _asbp_third_person_game_mode)
  (bind _outactors (`GameplayStatics.GetAllActorsOfClass` "/Game/Exam/DataAsset/BP_ExamPoint.BP_ExamPoint_C"))
  (bind _outactors_2 (`GameplayStatics.GetAllActorsOfClass` "/Game/Exam/DataAsset/BP_ExamPoison.BP_ExamPoison_C"))
  (bind _asbp_third_person_character (cast `/Game/ThirdPerson/Blueprints/BP_ThirdPersonCharacter` (`GameplayStatics.GetPlayerCharacter` 0)))
  (bind _output_get (set `/Game/ThirdPerson/Blueprints/BP_ThirdPersonCharacter.ExamTotalPoisonCollectibles` (`KismetArrayLibrary.Array_Length` _outactors_2) _asbp_third_person_character))
  (bind _output_get_2 (set `/Game/ThirdPerson/Blueprints/BP_ThirdPersonCharacter.ExamTotalPointsCollectibles` (`KismetArrayLibrary.Array_Length` _outactors) _asbp_third_person_character))
  (set `/Game/ThirdPerson/Blueprints/BP_ThirdPersonCharacter.ExamTotalCollectibles` (+ _output_get_2 _output_get) _asbp_third_person_character))

(fn `UserConstructionScript`)